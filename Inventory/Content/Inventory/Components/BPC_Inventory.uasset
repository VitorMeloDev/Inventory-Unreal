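; BPC_Inventory is a player component that manages money pickups, health and the inventory screen.
; On start it adds the input mapping, creates inventory and health bar widgets, and binds to the character capsule's overlap.
; Overlapped BP_Money actors add their DT_Money row amount to the total, update the widget and are destroyed.
; IA_Inventory opens the inventory in UI-only mode, while N and M keys raise and lower health, refreshing the bar.
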(event EventBeginPlay
  (CallFunction|OnStart))

(event EventTick
  (params (DeltaSeconds :type Float%20%28single-precision%29)))

(event Input|KeyboardEvents|N
  (params (Key :type Key%20Structure :default "None"))
  (:Pressed
    (CallFunction|IncreaseHealth 0.5)))

(event Input|KeyboardEvents|M
  (params (Key :type Key%20Structure :default "None"))
  (:Pressed
    (CallFunction|DecreaseHealth 0.5)))

(event Input|EnhancedActionEvents|EnhancedInputActionIA_Inventory
  (params (ActionValue :type Boolean) (ElapsedSeconds :type Float%20%28double-precision%29) (TriggeredSeconds :type Float%20%28double-precision%29) (InputAction :type Input%20Action%20Object%20Reference :default "/Game/Inventory/Inputs/IA_Inventory.IA_Inventory"))
  (bind _returnvalue (Game|GetPlayerController 0))
  (bind _inventorywidget (Variables|Widget|GetInventoryWidget))
  (UserInterface|Viewport|AddtoViewport _inventorywidget 0)
  (Variables|/Script/Engine.PlayerController|SetbShowMouseCursor _returnvalue true)
  (Input|SetInputModeUIOnly _returnvalue _inventorywidget "DoNotLock" false))

(fn OnStart
  (Input|AddMappingContext (PlayerController|LocalPlayerSubsystems|GetEnhancedInputLocalPlayerSubsystem (Game|GetPlayerController 0)) "/Game/Inventory/Inputs/IMC_Inventory.IMC_Inventory" 0 "(bIgnoreAllPressedKeysUntilRelease=True,bForceImmediately=False,bNotifyUserSettings=False)")
  (bind _returnvalue (UserInterface|CreateWidget "/Game/Inventory/UI/Widgtes/Inventory/WBP_Inventory.WBP_Inventory_C"))
  (Variables|Widget|SetInventoryWidget _returnvalue)
  (bind _asbp_third_person_character (Utilities|Casting|CastToBP_ThirdPersonCharacter (Game|GetPlayerCharacter 0)))
  (bind _output_get (Variables|Default|SetCharacter _asbp_third_person_character))
  (Collision|BindEventtoOnComponentBeginOverlap (Variables|/Script/Engine.Character|GetCapsuleComponent _output_get) (EventDispatchers|CreateEvent :!event PickUp))
  (bind _returnvalue_2 (UserInterface|CreateWidget "/Game/Inventory/UI/Widgtes/Inventory/WBP_HealthBar.WBP_HealthBar_C"))
  (bind _output_get_2 (Variables|Widget|SetHealthBarWidget _returnvalue_2))
  (Class|UserWidget|SetPositioninViewport _output_get_2 "(X=5.000000,Y=5.000000)" true)
  (UserInterface|Viewport|AddtoViewport _output_get_2 0))

(fn PickUp
  (params (OverlappedComponent :type Primitive%20Component%20Object%20Reference) (OtherActor :type Actor%20Object%20Reference) (OtherComp :type Primitive%20Component%20Object%20Reference) (OtherBodyIndex :type Integer) (bFromSweep :type Boolean) (SweepResult :type Hit%20Result%20Structure%20%28by%20ref%29))
  (bind _asbp_money (Utilities|Casting|CastToBP_Money OtherActor))
  (bind _returnvalue (Utilities|GetDataTableRow "/Game/Inventory/DataTable/DT_Money.DT_Money" (.rowname (Variables|/Game/Inventory/Blueprints/Money/BP_Money.BP_Money_C|GetDataTable _asbp_money)))
    (:then
      (bind _output_get (Variables|Money|SetMoneyComponent (+ (Variables|Money|GetMoneyComponent) (.amount _returnvalue))))
      (Variables|/Game/Inventory/UI/Widgtes/Inventory/WBP_Inventory.WBP_Inventory_C|SetMoneyAmountWidget (Variables|Widget|GetInventoryWidget) _output_get)
      (Actor|DestroyActor _asbp_money)
      (return))))

(fn IncreaseHealth
  (params (AmountToIncrease :type Float%20%28double-precision%29))
  (if (< (Variables|Health|GetHealth) (Variables|Health|GetMaxHealth))
    (Variables|Health|SetHealth (+ (Variables|Health|GetHealth) AmountToIncrease))
    (Default|UpdateHealthBar (Variables|Widget|GetHealthBarWidget))))

(fn DecreaseHealth
  (params (AmountToDecrease :type Float%20%28double-precision%29))
  (Variables|Health|SetHealth (- (Variables|Health|GetHealth) AmountToDecrease))
  (Default|UpdateHealthBar (Variables|Widget|GetHealthBarWidget)))